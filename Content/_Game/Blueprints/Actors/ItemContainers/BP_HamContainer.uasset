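; BP_HamContainer is an item container actor for ham that toggles a custom-depth marking on its container mesh when overlapped.
; Overlap begin enables custom depth with a fixed stencil value, and overlap end disables it and resets the stencil, with no filtering on the other actor.
; The construction script rebuilds the ItemMeshes array from the static mesh components attached directly under ContainerMesh.
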(event `self.ReceiveActorBeginOverlap`
  (params (OtherActor :type "Actor Object Reference"))
  (bind _containermesh (`self.ContainerMesh`))
  (`PrimitiveComponent.SetRenderCustomDepth` _containermesh true)
  (`PrimitiveComponent.SetCustomDepthStencilValue` _containermesh 252))

(event `self.ReceiveActorEndOverlap`
  (params (OtherActor :type "Actor Object Reference"))
  (bind _containermesh (`self.ContainerMesh`))
  (`PrimitiveComponent.SetRenderCustomDepth` _containermesh false)
  (`PrimitiveComponent.SetCustomDepthStencilValue` _containermesh 0))

(fn `UserConstructionScript`
  (`KismetArrayLibrary.Array_Clear` (`self.ItemMeshes`))
  (for _array_element (`SceneComponent.GetChildrenComponents` (`self.ContainerMesh`) false)
    (bind _asstatic_mesh_component (cast `StaticMeshComponent` _array_element))
    (`KismetArrayLibrary.Array_Add` (`self.ItemMeshes`) _asstatic_mesh_component)))