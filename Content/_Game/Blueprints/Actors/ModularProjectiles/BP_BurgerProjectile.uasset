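; Modular burger projectile whose child components under Mesh form a stack along local Y, apparently meant to close up when layers are hidden.
; Construction caches the static mesh children in ItemMeshes, while BeginPlay reverses the child list and records the Y spacing between neighbors.
; Test then repositions visible children using those spacings, indexed by a running visible count.
; Debug prints and disconnected copies of both loops suggest work in progress.
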(event `self.ReceiveBeginPlay`
  (bind _output_get (set `self.Children_0` (`SceneComponent.GetChildrenComponents` (`self.Mesh`) false)))
  (`KismetArrayLibrary.Array_Reverse` _output_get)
  (for (_array_element _array_index) (`self.Children_0`)
    (if (> _array_index 0)
      (bind (_relativelocation_x _relativelocation_y) (`KismetMathLibrary.BreakVector` (`SceneComponent.RelativeLocation` _array_element)))
      (bind (_relativelocation_x_2 _relativelocation_y_2) (`KismetMathLibrary.BreakVector` (`SceneComponent.RelativeLocation` (`|GetArrayItem` (`self.Children_0`) (- _array_index 1)))))
      (bind _returnvalue (- _relativelocation_y _relativelocation_y_2))
      (`KismetArrayLibrary.Array_Add` (`self.Distances`) _returnvalue)
      (`KismetSystemLibrary.PrintString` (`KismetStringLibrary.Concat_StrStr` (`KismetStringLibrary.Conv_IntToString` _array_index) " : " (`KismetSystemLibrary.GetDisplayName` _array_element) " : " (`KismetStringLibrary.Conv_DoubleToString` _returnvalue)) true true (struct :`G` 0.66 :`B` 1.0 :`A` 1.0) 360.0)
      (else
        (bind (_relativelocation_x_3 _relativelocation_y_3) (`KismetMathLibrary.BreakVector` (`SceneComponent.RelativeLocation` _array_element)))
        (`KismetArrayLibrary.Array_Add` (`self.Distances`) _relativelocation_y_3)
        (`KismetSystemLibrary.PrintString` (`KismetStringLibrary.Concat_StrStr` (`KismetStringLibrary.Conv_IntToString` 0) " : " (`KismetSystemLibrary.GetDisplayName` _array_element) " : " (`KismetStringLibrary.Conv_DoubleToString` _relativelocation_y_3)) true true (struct :`G` 0.66 :`B` 1.0 :`A` 1.0) 360.0))))
  (`self.Test`))

(event `Test`
  (bind (_relativelocation_x _relativelocation_y) (`KismetMathLibrary.BreakVector` (`SceneComponent.RelativeLocation` (`|GetArrayItem` (`self.Children_0`) (`self.TestCount`)))))
  (bind _returnvalue (+ _relativelocation_y (`|GetArrayItem` (`self.Distances`) (`self.TestCount`))))
  (set `self.TestCount` 0)
  (for (_array_element _array_index) (`self.Children_0`)
    (if (> _array_index 0)
      (if (`SceneComponent.IsVisible` _array_element)
        (bind (_relativelocation_x_2 _relativelocation_y_2 _relativelocation_z) (`KismetMathLibrary.BreakVector` (`SceneComponent.RelativeLocation` _array_element)))
        (`SceneComponent.K2_SetRelativeLocation` _array_element (`KismetMathLibrary.MakeVector` _relativelocation_x_2 _returnvalue _relativelocation_z) false false)
        (`/Engine/EditorBlueprintResources/StandardMacros.IncrementInt` (`self.TestCount`)
          (:`  `
            (`KismetSystemLibrary.PrintString` (`KismetStringLibrary.Concat_StrStr` (`KismetSystemLibrary.GetDisplayName` _array_element) ": " (`KismetStringLibrary.Conv_DoubleToString` _returnvalue)) true true (struct :`R` 1.0 :`G` 0.05098 :`A` 1.0) 360.0))))
      (elif (`SceneComponent.IsVisible` _array_element)
        (`/Engine/EditorBlueprintResources/StandardMacros.IncrementInt` (`self.TestCount`)
          (:`  `
            (bind (_relativelocation_x_3 _relativelocation_y_3) (`KismetMathLibrary.BreakVector` (`SceneComponent.RelativeLocation` _array_element)))
            (`KismetSystemLibrary.PrintString` (`KismetStringLibrary.Concat_StrStr` (`KismetSystemLibrary.GetDisplayName` _array_element) ": " (`KismetStringLibrary.Conv_DoubleToString` _relativelocation_y_3)) true true (struct :`R` 1.0 :`G` 0.05098 :`A` 1.0) 360.0)))))))

(fn `UserConstructionScript`
  (`KismetArrayLibrary.Array_Clear` (`self.ItemMeshes`))
  (for _array_element (`SceneComponent.GetChildrenComponents` (`self.Mesh`) false)
    (bind _asstatic_mesh_component (cast `StaticMeshComponent` _array_element))
    (`KismetArrayLibrary.Array_Add` (`self.ItemMeshes`) _asstatic_mesh_component)))