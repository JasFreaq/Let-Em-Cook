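; BP_OrderScreen is an in-world screen actor that shows the current dish orders to remote players through a widget component.
; On the server it binds to the GameplayGameMode's order added and removed delegates, then reports itself initialized after a short delay.
; Order changes are relayed by multicast events.
; Remote instances translate burger and roasted dinner orders into dish IDs and add or remove them on the WBP_DishOrderHandler widget.
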(event `self.ReceiveBeginPlay`
  (bind _returnvalue (`GameplayStatics.GetGameMode`))
  (`/Engine/EditorBlueprintResources/ActorMacros.Switch Has Authority`
    (:`Authority`
      (`/Engine/EditorBlueprintResources/StandardMacros.IsValid` _returnvalue
        (:`Is Valid`
          (bind _asgameplay_game_mode (cast `GameplayGameMode` _returnvalue))
          (add `GameplayGameMode.OrderAddedDelegate` _asgameplay_game_mode (delegate `On Order Added`))
          (add `GameplayGameMode.OrderRemovedDelegate` _asgameplay_game_mode (delegate `On Order Removed`))
          (`KismetSystemLibrary.Delay` 5.0)
          (`GameplayGameMode.OrderScreenInitialized` _asgameplay_game_mode))))
    (:`Remote`
      (bind _aswbp_dish_order_handler (cast `/Game/_Game/Blueprints/UserInterface/WBP_DishOrderHandler` (`WidgetComponent.GetWidget` (`self.Order Widget`))))
      (set `self.Dish Order Handler` _aswbp_dish_order_handler))))

(event `On Order Added`
  (params (Order :type "OrderInfoData Object Reference"))
  (`self.Multicast_OrderAdded` Order))

(event `On Order Removed`
  (params (Order :type "OrderInfoData Object Reference"))
  (`self.Multicast_OrderRemoved` Order))

(event `Multicast_OrderAdded`
  (params (`New Order` :type "OrderInfoData Object Reference"))
  (bind _dish_order_handler (`self.Dish Order Handler`))
  (`/Engine/EditorBlueprintResources/ActorMacros.Switch Has Authority`
    (:`Remote`
      (if (== `New Order` "/Game/_Game/DataAssets/OrderInfos/OI_Burger.OI_Burger")
        (`/Game/_Game/Blueprints/UserInterface/WBP_DishOrderHandler.AddDishToHandler` _dish_order_handler 1)
        (elif (== `New Order` "/Game/_Game/DataAssets/OrderInfos/OI_RoastedDinner.OI_RoastedDinner")
          (`/Game/_Game/Blueprints/UserInterface/WBP_DishOrderHandler.AddDishToHandler` _dish_order_handler 2))))))

(event `Multicast_OrderRemoved`
  (params (`Removed Order` :type "OrderInfoData Object Reference"))
  (bind _dish_order_handler (`self.Dish Order Handler`))
  (`/Engine/EditorBlueprintResources/ActorMacros.Switch Has Authority`
    (:`Remote`
      (if (== `Removed Order` "/Game/_Game/DataAssets/OrderInfos/OI_Burger.OI_Burger")
        (`/Game/_Game/Blueprints/UserInterface/WBP_DishOrderHandler.RemoveDishFromHandler` _dish_order_handler 1)
        (elif (== `Removed Order` "/Game/_Game/DataAssets/OrderInfos/OI_RoastedDinner.OI_RoastedDinner")
          (`/Game/_Game/Blueprints/UserInterface/WBP_DishOrderHandler.RemoveDishFromHandler` _dish_order_handler 2))))))

(fn `UserConstructionScript`)