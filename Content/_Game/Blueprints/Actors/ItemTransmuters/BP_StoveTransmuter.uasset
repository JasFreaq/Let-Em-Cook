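; BP_StoveTransmuter is a stove item transmuter that shows a timer widget for its transmutation progress.
; On BeginPlay it caches the BP_TransmuterTimer widget and takes the first BP_CharacterBase found as the look-at target.
; Each tick it feeds the remaining process time ratio into the widget and rotates the widget component toward that character.
; The timer is visible only while transmuting and collapsed otherwise.
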(event `self.ReceiveBeginPlay`
  (bind _asbp_transmuter_timer (cast `/Game/_Game/Blueprints/UserInterface/BP_TransmuterTimer` (`WidgetComponent.GetWidget` (`self.StoveTimer_Widget`))))
  (set `self.As BP Transmuter Timer` _asbp_transmuter_timer)
  (bind _outactors (`GameplayStatics.GetAllActorsOfClass` "/Game/_Game/Blueprints/Characters/BP_CharacterBase.BP_CharacterBase_C"))
  (set `self.LookAtTarget` (`|GetArrayItem` _outactors)))

(event `self.ReceiveTick`
  (params (DeltaSeconds :type "Float (single-precision)"))
  (bind _as_bp_transmuter_timer (`self.As BP Transmuter Timer`))
  (`/Engine/EditorBlueprintResources/StandardMacros.IsValid` (`self.As BP Transmuter Timer`)
    (:`Is Valid`
      (`self.UpdateTimer`)
      (`self.LookAtPlayers`)
      (if (`self.IsCurrentlyTransmuting`)
        (`Widget.SetVisibility` _as_bp_transmuter_timer "Visible")
        (else
          (`Widget.SetVisibility` _as_bp_transmuter_timer "Collapsed"))))))

(event `LookAtPlayers`
  (bind _lookattarget (`self.LookAtTarget`))
  ;[1 1 1] Rotate towards player
  (`/Engine/EditorBlueprintResources/StandardMacros.IsValid` _lookattarget
    (:`Is Valid`
      (`SceneComponent.K2_SetWorldRotation` (`self.StoveTimer_Widget`) (`KismetMathLibrary.FindLookAtRotation` (`self.K2_GetActorLocation`) (`self.K2_GetActorLocation` _lookattarget)) false false))))

(event `UpdateTimer`
  ;[1 1 1] Input max and current timer here pretty please uWu
  (set `/Game/_Game/Blueprints/UserInterface/BP_TransmuterTimer.Current Timer Ratio` (`self.GetProcessTimeRemainingRatio`) (`self.As BP Transmuter Timer`)))

(fn `UserConstructionScript`)