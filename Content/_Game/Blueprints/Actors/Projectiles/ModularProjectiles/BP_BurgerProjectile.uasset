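; Burger projectile Blueprint, one of the modular projectiles, built from item meshes attached under Mesh.
; Its construction script rebuilds the ItemMeshes array from Mesh's direct static mesh children.
; BeginPlay and Test are empty; leftover disconnected graph code measures Y gaps between children and restacks visible ones with debug prints, but never runs.
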(event `self.ReceiveBeginPlay`)

(event `Test`)

(fn `UserConstructionScript`
  (`KismetArrayLibrary.Array_Clear` (`self.ItemMeshes`))
  (for _array_element (`SceneComponent.GetChildrenComponents` (`self.Mesh`) false)
    (bind _asstatic_mesh_component (cast `StaticMeshComponent` _array_element))
    (`KismetArrayLibrary.Array_Add` (`self.ItemMeshes`) _asstatic_mesh_component)))